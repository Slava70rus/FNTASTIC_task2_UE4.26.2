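; BP_Socket is an actor that acts as a spawn point for a running AI NPC.
; SpawnRunner spawns a BP_NPC slightly offset from its Cube component, gives it a default controller, and calls Run with the socket's Point and BT variables.
; Three seconds later it ends the trails on its ParticleSystem component.
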(event `SpawnRunner`
  (bind _returnvalue (`|SpawnActorFromClass` "/Game/AI/BP_NPC.BP_NPC_C" (`KismetMathLibrary.MakeTransform` (+ (`SceneComponent.K2_GetComponentLocation` (`self.Cube`)) (0.0 30.0 0.0))) "Undefined" "OverrideRootScale" null null))
  (`Pawn.SpawnDefaultController` _returnvalue)
  (`/Game/AI/BP_NPC.Run` _returnvalue (`self.Point`) (`self.BT`))
  (`KismetSystemLibrary.Delay` 3.0)
  (`ParticleSystemComponent.EndTrails` (`self.ParticleSystem`)))

(fn `UserConstructionScript`)